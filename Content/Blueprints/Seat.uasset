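; Seat is an interactable prop that shows a remark when the mouse cursor hovers over its static mesh.
; BeginPlay enables mouse-over events on the player controller.
; Hovering enables input, adds a WB_Display_Text widget saying the player shouldn't sit right now, and turns on custom depth rendering for the mesh.
; Leaving disables input, removes all widgets and turns custom depth off.
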(event `self.ReceiveBeginPlay`
  (set `PlayerController.bEnableMouseOverEvents` true (`GameplayStatics.GetPlayerController` 0)))

(event `self.StaticMesh.OnBeginCursorOver`
  (params (TouchedComponent :type "PrimitiveComponent Object Reference"))
  (bind _returnvalue (`GameplayStatics.GetPlayerController` 0))
  (`|ExecutionSequence`
    (:`then_0`
      (`self.EnableInput` _returnvalue)
      (bind _returnvalue_2 (`|CreateWidget` "/Game/Blueprints/WB_Display_Text.WB_Display_Text_C" _returnvalue))
      (set `/Game/Blueprints/WB_Display_Text.PassedText` "I don't think I should be sitting right now." _returnvalue_2)
      (`UserWidget.AddToViewport` _returnvalue_2 0))
    (:`then_1`
      (`PrimitiveComponent.SetRenderCustomDepth` (`self.StaticMesh`) true))))

(event `self.StaticMesh.OnEndCursorOver`
  (params (TouchedComponent :type "PrimitiveComponent Object Reference"))
  (`|ExecutionSequence`
    (:`then_0`
      (`self.DisableInput` (`GameplayStatics.GetPlayerController` 0))
      (`WidgetLayoutLibrary.RemoveAllWidgets`))
    (:`then_1`
      (`PrimitiveComponent.SetRenderCustomDepth` (`self.StaticMesh`) false))))

(fn `UserConstructionScript`)
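; Elevator actor with two sliding doors that the player opens by pressing E while inside its Box trigger.
; Overlap enables input and shows an interact prompt widget; leaving disables input, removes all widgets and closes the doors after a delay.
; RightDoor and LeftDoor timelines drive the door positions, played to open and reversed to close.
; A SoundPlaying flag stops the pitch-randomized opening sound repeating until shortly after closing starts.
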(event `self.Box.OnComponentBeginOverlap`
  (params (OverlappedComponent :type "PrimitiveComponent Object Reference") (OtherActor :type "Actor Object Reference") (OtherComp :type "PrimitiveComponent Object Reference") (OtherBodyIndex :type Integer) (bFromSweep :type Boolean) (SweepResult :type "HitResult Structure (by ref)"))
  (bind _returnvalue (`GameplayStatics.GetPlayerController` 0))
  (`self.EnableInput` _returnvalue)
  (bind _returnvalue_2 (`|CreateWidget` "/Game/Blueprints/WB_Display_Text.WB_Display_Text_C" _returnvalue))
  (set `/Game/Blueprints/WB_Display_Text.PassedText` "Press E to interact" _returnvalue_2)
  (`UserWidget.AddToViewport` _returnvalue_2 0))

(event `self.Box.OnComponentEndOverlap`
  (params (OverlappedComponent :type "PrimitiveComponent Object Reference") (OtherActor :type "Actor Object Reference") (OtherComp :type "PrimitiveComponent Object Reference") (OtherBodyIndex :type Integer))
  (`|ExecutionSequence`
    (:`then_0`
      (`self.DisableInput` (`GameplayStatics.GetPlayerController` 0))
      (`WidgetLayoutLibrary.RemoveAllWidgets`))
    (:`then_1`
      (`KismetSystemLibrary.Delay` 1.0)
      ;[1 1 1] Play animation of door close and open on E press
      (`|ExecutionSequence`
        (:`then_0`
          (bind (_direction _newtrack_0) (`Timeline|Right Door` :!via `Reverse` :!label _label)
            (:`Update`
              (`SceneComponent.K2_SetRelativeLocation` (`self.DoorRight`) _newtrack_0 false false))))
        (:`then_1`
          (bind (_direction_2 _newtrack_0_2) (`Timeline|Left Door` :!via `Reverse` :!label _label_2)
            (:`Update`
              (`SceneComponent.K2_SetRelativeLocation` (`self.DoorLeft`) _newtrack_0_2 false false))))
        (:`then_2`
          (`KismetSystemLibrary.Delay` 1.0)
          (set `self.soundPlaying` false))))))

(event `Key|E`
  (params (Key :type "Key Structure"))
  ;[1 1 1] Play animation of door close and open on E press
  (:`Pressed`
    (`|ExecutionSequence`
      (:`then_0`
        (if (not (`self.soundPlaying`))
          (`GameplayStatics.PlaySoundAtLocation` "/Game/120557__mredig__elevator-door-open.120557__mredig__elevator-door-open" (`SceneComponent.K2_GetComponentLocation` (`self.DoorLeft`)) (struct) 1.0 (`KismetMathLibrary.RandomFloatInRange` 0.9 1.0)))
        (`|ExecutionSequence`
          (:`then_0`
            (goto _label))
          (:`then_1`
            (set `self.soundPlaying` true))))
      (:`then_1`
        (goto _label_2)))))

(fn `UserConstructionScript`)
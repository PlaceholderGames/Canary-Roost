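; BP_Door is an interactable glass door that swings open when E is pressed inside its trigger, then closes automatically.
; Trigger overlap enables player input and shows a WB_Display_Text prompt; leaving disables input and removes all widgets.
; Pressing E plays a timeline driving the door's yaw, and releasing E reverses it after a delay.
; Open and close sounds spawn at world origin rather than at the door.
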(event `self.DoorTrigger.OnComponentBeginOverlap`
  (params (OverlappedComponent :type "PrimitiveComponent Object Reference") (OtherActor :type "Actor Object Reference") (OtherComp :type "PrimitiveComponent Object Reference") (OtherBodyIndex :type Integer) (bFromSweep :type Boolean) (SweepResult :type "HitResult Structure (by ref)"))
  (bind _returnvalue (`GameplayStatics.GetPlayerController` 0))
  (`self.EnableInput` _returnvalue)
  (bind _returnvalue_2 (`|CreateWidget` "/Game/Blueprints/WB_Display_Text.WB_Display_Text_C" _returnvalue))
  (set `/Game/Blueprints/WB_Display_Text.PassedText` "Press E to interact" _returnvalue_2)
  (`UserWidget.AddToViewport` _returnvalue_2 0))

(event `self.DoorTrigger.OnComponentEndOverlap`
  (params (OverlappedComponent :type "PrimitiveComponent Object Reference") (OtherActor :type "Actor Object Reference") (OtherComp :type "PrimitiveComponent Object Reference") (OtherBodyIndex :type Integer))
  (`self.DisableInput` (`GameplayStatics.GetPlayerController` 0))
  (`WidgetLayoutLibrary.RemoveAllWidgets`))

(event `Key|E`
  (params (Key :type "Key Structure"))
  ;[1 1 1] Play animation of door close and open on E press
  (:`Pressed`
    (`GameplayStatics.SpawnSoundAtLocation` "/Game/Sounds/glass-door-open-1.glass-door-open-1")
    (bind (_direction _door_open) (`Timeline|DoorRoatation` :!label _label)
      (:`Update`
        (`SceneComponent.K2_SetRelativeRotation` (`self.Door`) (`KismetMathLibrary.MakeRotator` 0.0 0.0 _door_open) false false))
      (:`Finished`
        (`GameplayStatics.SpawnSoundAtLocation` "/Game/Sounds/glass-door-close-1.glass-door-close-1"))))
  (:`Released`
    (`KismetSystemLibrary.Delay` 2.5)
    (goto _label :!via `Reverse`)))

(fn `UserConstructionScript`)
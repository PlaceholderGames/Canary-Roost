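; BP_LaptopUseless is a non-functional laptop prop in the hacking content that tells the player it doesn't seem to work.
; Overlapping its Box enables input, shows a WB_Display_Text message and turns on custom depth on the DoorFrame component, likely for highlighting.
; Leaving disables input, removes all widgets, not just its own, and clears custom depth.
; Neither overlap event checks which actor triggered it.
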(event `self.ReceiveBeginPlay`
  (set `PlayerController.bEnableMouseOverEvents` true (`GameplayStatics.GetPlayerController` 0)))

(event `self.Box.OnComponentBeginOverlap`
  (params (OverlappedComponent :type "PrimitiveComponent Object Reference") (OtherActor :type "Actor Object Reference") (OtherComp :type "PrimitiveComponent Object Reference") (OtherBodyIndex :type Integer) (bFromSweep :type Boolean) (SweepResult :type "HitResult Structure (by ref)"))
  (bind _returnvalue (`GameplayStatics.GetPlayerController` 0))
  (`|ExecutionSequence`
    (:`then_0`
      (`self.EnableInput` _returnvalue)
      (bind _returnvalue_2 (`|CreateWidget` "/Game/Blueprints/WB_Display_Text.WB_Display_Text_C" _returnvalue))
      (set `/Game/Blueprints/WB_Display_Text.PassedText` "Doesn't seem to work." _returnvalue_2)
      (`UserWidget.AddToViewport` _returnvalue_2 0))
    (:`then_1`
      (`PrimitiveComponent.SetRenderCustomDepth` (`self.DoorFrame`) true))))

(event `self.Box.OnComponentEndOverlap`
  (params (OverlappedComponent :type "PrimitiveComponent Object Reference") (OtherActor :type "Actor Object Reference") (OtherComp :type "PrimitiveComponent Object Reference") (OtherBodyIndex :type Integer))
  (`|ExecutionSequence`
    (:`then_0`
      (`self.DisableInput` (`GameplayStatics.GetPlayerController` 0))
      (`WidgetLayoutLibrary.RemoveAllWidgets`))
    (:`then_1`
      (`PrimitiveComponent.SetRenderCustomDepth` (`self.DoorFrame`) false))))

(fn `UserConstructionScript`)
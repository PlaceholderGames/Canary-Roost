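; LevelElevator is an elevator Blueprint with two sliding doors that the player can open once MinigameCompleted is true.
; Overlapping its Box enables input and shows a "Press 'E' to open" widget; leaving disables input and removes all widgets.
; Pressing E plays two Timelines that move the left and right doors, and releasing it reverses both after a short delay to close them.
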(event `self.Box.OnComponentBeginOverlap`
  (params (OverlappedComponent :type "PrimitiveComponent Object Reference") (OtherActor :type "Actor Object Reference") (OtherComp :type "PrimitiveComponent Object Reference") (OtherBodyIndex :type Integer) (bFromSweep :type Boolean) (SweepResult :type "HitResult Structure (by ref)"))
  (bind _returnvalue (`GameplayStatics.GetPlayerController` 0))
  (if (`self.MinigameCompleted?`)
    (`self.EnableInput` _returnvalue)
    (bind _returnvalue_2 (`|CreateWidget` "/Game/Blueprints/WB_Display_Text.WB_Display_Text_C" _returnvalue))
    (set `/Game/Blueprints/WB_Display_Text.PassedText` "Press 'E' to open" _returnvalue_2)
    (`UserWidget.AddToViewport` _returnvalue_2 0)))

(event `self.Box.OnComponentEndOverlap`
  (params (OverlappedComponent :type "PrimitiveComponent Object Reference") (OtherActor :type "Actor Object Reference") (OtherComp :type "PrimitiveComponent Object Reference") (OtherBodyIndex :type Integer))
  (`self.DisableInput` (`GameplayStatics.GetPlayerController` 0))
  (`WidgetLayoutLibrary.RemoveAllWidgets`))

(event `Key|E`
  (params (Key :type "Key Structure"))
  (bind _minigamecompleted_ (`self.MinigameCompleted?`))
  (:`Pressed`
    ;[1 1 1] Play animation of door close and open on E press
    (if _minigamecompleted_
      (`|ExecutionSequence`
        (:`then_0`
          (bind (_direction _newtrack_1) (`Timeline|Timeline_0` :!label _label)
            (:`Update`
              (`SceneComponent.K2_SetRelativeLocation` (`self.DoorRight`) _newtrack_1 false false))))
        (:`then_1`
          (bind (_direction_2 _newtrack_1_2) (`Timeline|Timeline_1` :!label _label_2)
            (:`Update`
              (`SceneComponent.K2_SetRelativeLocation` (`self.DoorLeft`) _newtrack_1_2 false false)))))))
  (:`Released`
    (if _minigamecompleted_
      (`KismetSystemLibrary.Delay` 2.0)
      (`|ExecutionSequence`
        (:`then_0`
          (goto _label :!via `Reverse`))
        (:`then_1`
          (goto _label_2 :!via `Reverse`))))))

(fn `UserConstructionScript`)